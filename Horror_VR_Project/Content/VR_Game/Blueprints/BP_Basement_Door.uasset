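; Keycard-locked basement door for the VR game that swings open once unlocked and approached by the player.
; Overlapping the reader box with the assigned key actor unlocks the door, cracks it ajar, adds audio, hides the reader highlight and reveals the handle mesh.
; Player pawn overlap with the door box then plays a sound and swings it wide via a timeline-scaled yaw.
; Rotation is ignored once fully open; doors starting unlocked apply an initial rotation.
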(event OnComponentBeginOverlap(doorOpenBox)
  (params (OverlappedComponent :type Primitive%20Component%20Object%20Reference) (OtherActor :type Actor%20Object%20Reference) (OtherComp :type Primitive%20Component%20Object%20Reference) (OtherBodyIndex :type Integer) (bFromSweep :type Boolean) (SweepResult :type Hit%20Result%20Structure%20%28by%20ref%29))
  ;[1 1 1] Door Collitision
  (CallFunction|CheckDoorOverlap -95.0 OtherActor))

(event OnComponentBeginOverlap(readerBox)
  (params (OverlappedComponent :type Primitive%20Component%20Object%20Reference) (OtherActor :type Actor%20Object%20Reference) (OtherComp :type Primitive%20Component%20Object%20Reference) (OtherBodyIndex :type Integer) (bFromSweep :type Boolean) (SweepResult :type Hit%20Result%20Structure%20%28by%20ref%29))
  (bind _keytounlock (Variables|Default|GetkeyToUnlock))
  (bind _handletohighlight (Variables|Default|GetHandleToHighlight))
  (bind _returnvalue (== OtherActor _keytounlock))
  ;[1 1 1] unlock with keycard
  (Utilities|String|LogString "Reader overlap!")
  (Utilities|String|LogString (Utilities|GetDisplayName OtherActor))
  (Utilities|String|LogString (Utilities|GetDisplayName _keytounlock))
  (Utilities|String|LogString (Utilities|String|ToString(Boolean) _returnvalue))
  (Utilities|IsValid OtherActor
    (:Is%20Valid
      (if _returnvalue
        (CallFunction|UnlockDoor)
        (CallFunction|UnHighlightReader)
        (Utilities|IsValid _handletohighlight
          (:Is%20Valid
            (Rendering|SetVisibility (Variables|/Script/Engine.StaticMeshActor|GetStaticMeshComponent _handletohighlight) true false)))))))

(event Custom|unlock%20Door
  ;[1 1 1] unlock Door
  (Utilities|String|LogString "Unlocking dooooor!")
  (Variables|Default|SetisDoorUnlocked true)
  (CallFunction|RotateDoor -13.0)
  (AddComponent|AddAudioComponent false))

(event Custom|rotateDoor
  (params (rotation :type Float%20%28double-precision%29))
  ;[1 1 1] rotate Door
  (if (not (< (Variables|Default|GetcurrentRotation) -8e+01))
    (Variables|Default|SetcurrentRotation rotation)
    (bind _dooropenanim (Timeline|doorOpenAnim PlayFromStart)
      (:Update
        (Transformation|SetRelativeRotation (Variables|Default|GetSM_Door) (Math|Rotator|MakeRotator 0.0 0.0 (* _dooropenanim rotation)) false false)))))

(event Custom|checkDoorOverlap
  (params (rotation :type Float%20%28double-precision%29) (Actor :type Actor%20Object%20Reference%20%28by%20ref%29))
  ;[1 1 1] Check Overlap
  (if (== Actor (Game|Player|GetPlayerPawn 0))
    (if (Variables|Default|GetisDoorUnlocked)
      (if true
        (Audio|PlaySound2D "/Game/HorrorEngine/Audio/Elecronic/KeyCardOpen.KeyCardOpen" 1.0 1.0 0.0 0 0)
        (Utilities|String|LogString "Door opening now!")
        (CallFunction|RotateDoor rotation)))))

(event Custom|highlightReader
  (bind _highlight (Variables|Default|GetHighlight))
  ;[1 1 1] Highlight Unhilight KeycardReader
  (Utilities|IsValid _highlight
    (:Is%20Valid
      (Rendering|SetVisibility _highlight true false))))

(event Custom|unHighlightReader
  (bind _highlight (Variables|Default|GetHighlight))
  ;[1 1 1] Highlight Unhilight KeycardReader
  (Utilities|IsValid _highlight
    (:Is%20Valid
      (Rendering|SetVisibility _highlight false false))))

(event EventBeginPlay
  ;[1 1 1] Initialize door
  (if (Variables|Default|GetisDoorUnlocked)
    (CallFunction|RotateDoor (Variables|Default|GetinitalRotation))))

(fn ConstructionScript)