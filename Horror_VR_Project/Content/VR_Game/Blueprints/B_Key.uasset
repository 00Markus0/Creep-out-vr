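; B_Key is a key pickup actor in a VR game, with a configurable mesh and a highlight that can start on or off.
; Pickup events for specific keys hide the highlight and trigger story changes on actors passed in by the caller.
; The classroom key destroys the Dad, Mum and Creep actors after a delay.
; The office key unlocks the basement door and teleports the wandering creep to a hardcoded spot.
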(event Custom|classroomKeyPickedUp
  (params (parentsLeavingDuration :type Float%20%28double-precision%29) (Dad :type BP%20Dad%20Object%20Reference%20%28by%20ref%29) (Mum :type BP%20Mum%20Object%20Reference%20%28by%20ref%29) (Creep :type BP%20Creep%20Object%20Reference%20%28by%20ref%29))
  ;[1 1 1] Classroom
  (Utilities|String|LogString "Clasroom key picked up")
  (CallFunction|UnHighlightKeycard)
  (Utilities|FlowControl|Delay parentsLeavingDuration)
  (Utilities|IsValid Dad
    (:Is%20Valid
      (Actor|DestroyActor Dad)
      (Utilities|IsValid Mum
        (:Is%20Valid
          (Actor|DestroyActor Mum)
          (Utilities|IsValid Creep
            (:Is%20Valid
              (Actor|DestroyActor Creep))))))))

(event Custom|officeKeyPickedUp
  (params (doorToBasement :type BP%20Door%20Object%20Reference%20%28by%20ref%29) (WanderingCreep :type BP%20Creep%20Chase%20Object%20Reference%20%28by%20ref%29))
  ;[1 1 1] Office
  (CallFunction|UnHighlightKeycard)
  (Utilities|IsValid doorToBasement
    (:Is%20Valid
      (Default|UnlockDoor doorToBasement)
      (Utilities|IsValid WanderingCreep
        (:Is%20Valid
          (Transformation|SetActorLocationAndRotation WanderingCreep "55.000000,800.000000,96.000000" "0.000000,180.000000,0.000000" false true))))))

(event Custom|highlightKeycard
  ;[1 1 1] Highlight / Unhighlight Key
  (Rendering|SetVisibility (Variables|Default|GetHighlight) true false))

(event Custom|unHighlightKeycard
  ;[1 1 1] Highlight / Unhighlight Key
  (Rendering|SetVisibility (Variables|Default|GetHighlight) false false))

(event EventBeginPlay
  (if (Variables|Default|GetisHighlitedAtStart)
    (CallFunction|HighlightKeycard)
    (else
      (CallFunction|UnHighlightKeycard))))

(event Collision|EventActorBeginOverlap
  (params (OtherActor :type Actor%20Object%20Reference)))

(event EventTick
  (params (DeltaSeconds :type Float%20%28single-precision%29)))

(fn ConstructionScript
  (Components|StaticMesh|SetStaticMesh (Variables|Default|GetKeyMesh) (Variables|Default|GetMesh)))