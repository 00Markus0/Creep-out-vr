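; VR door lock Blueprint for a door that stays shut until its assigned key actor touches the lock box.
; A matching key unlocks it, adds an audio component, immediately triggers the full swing and highlights an optional light switch.
; Once unlocked, player overlap with the open box also requests that swing.
; A timeline scales the door mesh's yaw, with a rotation guard preventing replays after fully opening.
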(event OnComponentBeginOverlap(doorOpenBox)
  (params (OverlappedComponent :type Primitive%20Component%20Object%20Reference) (OtherActor :type Actor%20Object%20Reference) (OtherComp :type Primitive%20Component%20Object%20Reference) (OtherBodyIndex :type Integer) (bFromSweep :type Boolean) (SweepResult :type Hit%20Result%20Structure%20%28by%20ref%29))
  ;[1 1 1] Door Collitision
  (CallFunction|CheckDoorOverlap -95.0 OtherActor))

(event OnComponentBeginOverlap(lockBox)
  (params (OverlappedComponent :type Primitive%20Component%20Object%20Reference) (OtherActor :type Actor%20Object%20Reference) (OtherComp :type Primitive%20Component%20Object%20Reference) (OtherBodyIndex :type Integer) (bFromSweep :type Boolean) (SweepResult :type Hit%20Result%20Structure%20%28by%20ref%29))
  (bind _keytounlock (Variables|Default|GetkeyToUnlock))
  (bind _lightswitchtohighlight (Variables|Default|GetlightSwitchToHighlight))
  (bind _returnvalue (== OtherActor _keytounlock))
  ;[1 1 1] unlock with key
  (Utilities|String|LogString "Clasroom overlap!")
  (Utilities|String|LogString (Utilities|GetDisplayName 0))
  (Utilities|String|LogString (Utilities|GetDisplayName _keytounlock))
  (Utilities|String|LogString (Utilities|String|ToString(Boolean) _returnvalue))
  (Utilities|IsValid OtherActor
    (:Is%20Valid
      (if _returnvalue
        (if (not (Variables|Default|GetisDoorUnlocked))
          (CallFunction|UnlockDoor)
          (CallFunction|CheckDoorOverlap -95.0 (Game|Player|GetPlayerPawn 0))
          (Utilities|IsValid _lightswitchtohighlight
            (:Is%20Valid
              (Default|HighlightLightSwitch _lightswitchtohighlight))))))))

(event Custom|unlock%20Door
  ;[1 1 1] unlock Door
  (Variables|Default|SetisDoorUnlocked true)
  (CallFunction|RotateDoor -13.0)
  (AddComponent|AddAudioComponent false))

(event Custom|rotateDoor
  (params (rotation :type Float%20%28double-precision%29))
  ;[1 1 1] rotate Door
  (if (not (< (Variables|Default|GetcurrentRotation) -8e+01))
    (Variables|Default|SetcurrentRotation rotation)
    (bind _dooropenanim (Timeline|doorOpenAnim PlayFromStart)
      (:Update
        (Transformation|SetRelativeRotation (Variables|Default|GetSM_Door) (Math|Rotator|MakeRotator 0.0 0.0 (* _dooropenanim rotation)) false false)))))

(event Custom|checkDoorOverlap
  (params (rotation :type Float%20%28double-precision%29) (Actor :type Actor%20Object%20Reference%20%28by%20ref%29))
  ;[1 1 1] Check Overlap
  (if (== Actor (Game|Player|GetPlayerPawn 0))
    (if (Variables|Default|GetisDoorUnlocked)
      (CallFunction|RotateDoor rotation))))

(event EventBeginPlay
  ;[1 1 1] Initialize door
  (if (Variables|Default|GetisDoorUnlocked)
    (CallFunction|RotateDoor (Variables|Default|GetinitalRotation))))

(event EventTick
  (params (DeltaSeconds :type Float%20%28single-precision%29)))

(fn ConstructionScript)