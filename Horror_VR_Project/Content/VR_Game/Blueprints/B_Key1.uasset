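; B_Key1 is a keycard in the VR game with a Highlight component that marks it visually.
; At BeginPlay, the IsHighlitedAtStart flag decides whether the highlight is shown, using two events that toggle that component's visibility.
; The classroom pickup event hides the highlight, waits for the given parents-leaving duration, then destroys the Dad, Mum and Creep actors through nested validity checks.
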(event Custom|classroomKeyPickedUp
  (params (parentsLeavingDuration :type Float%20%28double-precision%29) (Dad :type BP%20Dad%20Object%20Reference%20%28by%20ref%29) (Mum :type BP%20Mum%20Object%20Reference%20%28by%20ref%29) (Creep :type BP%20Creep%20Arguing%20Object%20Reference%20%28by%20ref%29))
  ;[1 1 1] Classroom
  (CallFunction|UnHighlightKeycard)
  (Utilities|FlowControl|Delay parentsLeavingDuration)
  (Utilities|IsValid Dad
    (:Is%20Valid
      (Actor|DestroyActor Dad)
      (Utilities|IsValid Mum
        (:Is%20Valid
          (Actor|DestroyActor Mum)
          (Utilities|IsValid Creep
            (:Is%20Valid
              (Actor|DestroyActor Creep))))))))

(event Custom|highlightKeycard
  ;[1 1 1] Highlight / Unhighlight Key
  (Rendering|SetVisibility (Variables|Default|GetHighlight) true false))

(event Custom|unHighlightKeycard
  ;[1 1 1] Highlight / Unhighlight Key
  (Rendering|SetVisibility (Variables|Default|GetHighlight) false false))

(event EventBeginPlay
  (if (Variables|Default|GetisHighlitedAtStart)
    (CallFunction|HighlightKeycard)
    (else
      (CallFunction|UnHighlightKeycard))))

(fn ConstructionScript)