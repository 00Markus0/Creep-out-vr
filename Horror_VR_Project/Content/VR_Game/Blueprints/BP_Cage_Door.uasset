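; BP_Cage_Door is a keycard-locked cage door for the VR game.
; Overlapping the reader with the matching key unlocks the door, cracks it ajar, hides the reader highlight and, given a valid handle, reveals it and updates the objective hint.
; The player entering the door box then swings it wide via CloseDoor, despite that name, and clears the unlocked flag.
; A timeline scales the target yaw, and rotation stops responding once fully swung.
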(event OnComponentBeginOverlap(doorOpenBoxBasement)
  (params (OverlappedComponent :type Primitive%20Component%20Object%20Reference) (OtherActor :type Actor%20Object%20Reference) (OtherComp :type Primitive%20Component%20Object%20Reference) (OtherBodyIndex :type Integer) (bFromSweep :type Boolean) (SweepResult :type Hit%20Result%20Structure%20%28by%20ref%29))
  ;[1 1 1] Door Collision
  (CallFunction|CloseDoor -95.0 OtherActor))

(event OnComponentBeginOverlap(readerBox)
  (params (OverlappedComponent :type Primitive%20Component%20Object%20Reference) (OtherActor :type Actor%20Object%20Reference) (OtherComp :type Primitive%20Component%20Object%20Reference) (OtherBodyIndex :type Integer) (bFromSweep :type Boolean) (SweepResult :type Hit%20Result%20Structure%20%28by%20ref%29))
  (bind _handletohighlight (Variables|Default|GetHandleToHighlight))
  ;[1 1 1] unlock with keycard
  (Utilities|IsValid OtherActor
    (:Is%20Valid
      (if (not (Variables|Default|GetisDoorUnlocked))
        (if (== OtherActor (Variables|Default|GetkeyToUnlock))
          (CallFunction|UnlockDoor)
          (CallFunction|UnHighlightReader)
          (Utilities|IsValid _handletohighlight
            (:Is%20Valid
              (Rendering|SetVisibility (Variables|/Script/Engine.StaticMeshActor|GetStaticMeshComponent _handletohighlight) true false)
              (Utilities|UpdateHintText "Help your mum"))))))))

(event Custom|unlock%20Door
  ;[1 1 1] unlock Door
  (Variables|Default|SetisDoorUnlocked true)
  (CallFunction|RotateDoor -13.0)
  (Audio|PlaySound2D "/Game/HorrorEngine/Audio/DoorsAndFurnitures/Unlock02.Unlock02" 1.0 1.0 0.0 0 0)
  (Audio|PlaySound2D 0 1.0 1.0 0.0 0 0))

(event Custom|rotateDoor
  (params (rotation :type Float%20%28double-precision%29))
  ;[1 1 1] rotate Door
  (if (not (< (Variables|Default|GetcurrentPosition) -8e+01))
    (Variables|Default|SetcurrentPosition rotation)
    (bind _dooropenanim (Timeline|doorOpenAnim PlayFromStart)
      (:Update
        (Transformation|SetRelativeRotation (Variables|Default|GetSM_Door) (Math|Rotator|MakeRotator 0.0 0.0 (* _dooropenanim rotation)) false false)))))

(event Custom|closeDoor
  (params (rotation :type Float%20%28double-precision%29) (Actor :type Actor%20Object%20Reference%20%28by%20ref%29))
  ;[1 1 1] Check Overlap
  (if (== Actor (Game|Player|GetPlayerPawn 0))
    (if (Variables|Default|GetisDoorUnlocked)
      (CallFunction|RotateDoor rotation)
      (Audio|PlaySound2D "/Game/HorrorEngine/Audio/DoorsAndFurnitures/HandleOpen06.HandleOpen06" 1.0 1.0 0.0 0 0)
      (Variables|Default|SetisDoorUnlocked false))))

(event Custom|highlightReader
  (bind _readerhighlight (Variables|Default|GetReaderHighlight))
  ;[1 1 1] Highlight Unhilight KeycardReader
  (Utilities|IsValid _readerhighlight
    (:Is%20Valid
      (Rendering|SetVisibility _readerhighlight true false))))

(event Custom|unHighlightReader
  (bind _readerhighlight (Variables|Default|GetReaderHighlight))
  ;[1 1 1] Highlight Unhilight KeycardReader
  (Utilities|IsValid _readerhighlight
    (:Is%20Valid
      (Rendering|SetVisibility _readerhighlight false false))))

(event EventBeginPlay
  ;[1 1 1] Initialize door
  (if (Variables|Default|GetisDoorUnlocked)
    (CallFunction|RotateDoor (Variables|Default|GetinitalPosition))))

(fn ConstructionScript)