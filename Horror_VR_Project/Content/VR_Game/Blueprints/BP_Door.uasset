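; BP_Door is a door Blueprint in the VR game that swings open when an actor enters its trigger box.
; If unlocked, it rotates to its initial rotation on BeginPlay.
; Overlaps on DoorOpenBox pass through CheckDoorOverlap with the lock state, actor and current rotation, triggering a fixed-angle swing on success.
; The DoorOpenAnim timeline scales the target yaw to animate the door mesh, while CurrentRotation stores that target.
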(event OnComponentBeginOverlap(doorOpenBox)
  (params (OverlappedComponent :type Primitive%20Component%20Object%20Reference) (OtherActor :type Actor%20Object%20Reference) (OtherComp :type Primitive%20Component%20Object%20Reference) (OtherBodyIndex :type Integer) (bFromSweep :type Boolean) (SweepResult :type Hit%20Result%20Structure%20%28by%20ref%29))
  ;[1 1 1] Collision
  (Utilities|CheckDoorOverlap (Variables|Default|GetisDoorUnlocked) OtherActor (Variables|Default|GetcurrentRotation)
    (:Success
      (CallFunction|RotateDoor -95.0))))

(event Custom|rotateDoor
  (params (rotation :type Float%20%28double-precision%29))
  ;[1 1 1] rotate Door
  (Variables|Default|SetcurrentRotation rotation)
  (bind _dooropenanim (Timeline|doorOpenAnim PlayFromStart)
    (:Update
      (Transformation|SetRelativeRotation (Variables|Default|GetSM_Door) (Math|Rotator|MakeRotator 0.0 0.0 (* _dooropenanim rotation)) false false))))

(event EventBeginPlay
  ;[1 1 1] Initialize door
  (if (Variables|Default|GetisDoorUnlocked)
    (CallFunction|RotateDoor (Variables|Default|GetinitalRotation))))

(fn ConstructionScript)