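; Trigger actor in a VR game that starts the classroom key pickup sequence when the player pawn overlaps it.
; Each player overlap resets HMD position, and the first validated one notifies the key with the arguing Mum, Dad and Creep references.
; It also plays a wood sound and changes the hint to "Unlock the door".
; Once the hint updates, it latches and, after the parents' leaving delay, stops the arguing and wood sounds.
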(event Collision|EventActorBeginOverlap
  (params (OtherActor :type Actor%20Object%20Reference))
  (bind _returnvalue (Game|Player|GetPlayerPawn 0))
  (bind _woodsoundreference (Variables|Default|GetwoodSoundReference))
  (bind _audiocomponent (Variables|/Script/Engine.AmbientSound|GetAudioComponent _woodsoundreference))
  ;[1 1 1] Classroom Triggered
  (Development|PrintString "Overlap")
  (if (== OtherActor _returnvalue)
    (Utilities|Casting|CastToVRPawn _returnvalue)
    (Class|HeadMountedDisplayFunctionLibrary|ResetOrientationandPosition 0.0 "Position")
    (if (not (Variables|Default|GetisClassroomTriggered))
      (Utilities|ValidateAllVariables
        (:Success
          (Default|ClassroomKeyPickedUp (Variables|Default|GetClassroomKeyReference) (Variables|Default|GetparentsLeavingDuration) (Variables|Default|GetdadArguingReference) (Variables|Default|GetmumArguingReference) (Variables|Default|GetcreepArguingReference))
          (Audio|Components|Audio|Play _audiocomponent 0.0)
          (Utilities|UpdateHintText "Unlock the door"
            (:updated
              (Variables|Default|SetisClassroomTriggered true)
              (Utilities|FlowControl|Delay (Variables|Default|GetparentsLeavingDuration))
              (Audio|Components|Audio|Stop (Variables|/Script/Engine.AmbientSound|GetAudioComponent (Variables|Default|GetArguingSoundReference)))
              (Audio|Components|Audio|Stop _audiocomponent))))))))

(fn ConstructionScript)