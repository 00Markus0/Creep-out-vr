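; Trigger actor that runs the closing jump scare and ending of the VR demo when the player pawn overlaps it.
; It disables input, spawns a screaming BP_Creep with sounds, and drives the pawn's yaw with a timeline.
; It then teleports the player into a cage behind a blackscreen material fade, restores control and shows a thanks hint.
; After a delay, it disables control again, shows ending text and quits the game.
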(event Custom|endSequence
  (bind _returnvalue (Game|Player|GetPlayerPawn 0))
  ;[0.1651 0.1651 0.1651] Helper Events
  (Input|DisableInput _returnvalue 0)
  (bind _asvrpawn (Utilities|Casting|CastToVRPawn _returnvalue))
  (Default|DisableWalkingSound _asvrpawn)
  (Utilities|SetBlackScreenText (Variables|Default|GetText)
    (:Finished
      (CallFunction|AnimateBlackScreen)
      (Utilities|FlowControl|Delay 8.0)
      (Default|ToggleBlackScreen _asvrpawn)
      (Game|QuitGame 0 "Quit" false))))

(event Custom|playJumpScare
  (bind _returnvalue (Game|Player|GetPlayerPawn 0))
  ;[0.1651 0.1651 0.1651] Helper Events
  (Audio|PlaySound2D "/Game/VR_Game/Sounds/S_Scared_02.S_Scared_02" 1.0 1.0 0.0 0 0)
  (Audio|PlaySound2D "/Game/VR_Game/Sounds/SC_JumpScare.SC_JumpScare" 1.0 1.0 0.0 0 0)
  (Input|DisableInput _returnvalue 0)
  (bind _asvrpawn (Utilities|Casting|CastToVRPawn _returnvalue))
  (Default|DisableWalkingSound _asvrpawn)
  (bind _returnvalue_2 (Game|SpawnActorfromClass "/Game/MetaHumans/Creep/BP_Creep.BP_Creep_C" (Math|Transform|MakeTransform "1350.000000,3320.000000,-690.000000" "0.000000,-90.000000,0.000000" "1.000000,1.000000,1.000000") "AlwaysSpawn" 0 0))
  (Components|Animation|PlayAnimation (Variables|/Game/MetaHumans/Creep/BP_Creep.BP_Creep_C|GetFeet _returnvalue_2) "/Game/VR_Game/Animations/ZombieScream_UE.ZombieScream_UE" false)
  (Components|Animation|PlayAnimation (Variables|/Game/MetaHumans/Creep/BP_Creep.BP_Creep_C|GetBody _returnvalue_2) "/Game/VR_Game/Animations/ZombieScream_UE.ZombieScream_UE" false)
  (Components|Animation|PlayAnimation (Variables|/Game/MetaHumans/Creep/BP_Creep.BP_Creep_C|GetFace _returnvalue_2) "/Game/Cinematics/Takes/2023-05-29/Creep_Jumpscare_01_Subscenes/Animation/BP_Creep_Jumpscare_Creep_Jumpscare_01_0.BP_Creep_Jumpscare_Creep_Jumpscare_01_0" true)
  (Utilities|FlowControl|Delay 0.6)
  (Audio|PlaySound2D "/Game/VR_Game/Sounds/S_Heartbeat1.S_Heartbeat1" 1.0 1.0 0.0 0 0))

(event Custom|animate%20BlackScreen
  ;[1 1 1] animate BlackScreen Widget
  (bind _asvrpawn (Utilities|Casting|CastToVRPawn (Game|Player|GetPlayerPawn 0)))
  (Class|HeadMountedDisplayFunctionLibrary|ResetOrientationandPosition 0.0 "OrientationAndPosition")
  (bind _returnvalue (Rendering|Material|CreateDynamicMaterialInstance (Variables|/Game/VRTemplate/Blueprints/VRPawn.VRPawn_C|GetBlackscreen _asvrpawn) 0 "/Game/VR_Game/Materials/ML_Black_Capsule.ML_Black_Capsule" "None" :!class /Script/Engine.PrimitiveComponent))
  (if (Variables|/Game/VRTemplate/Blueprints/VRPawn.VRPawn_C|GetblackscreenVisibility _asvrpawn)
    (bind _opacity_track (Timeline|Opacity ReverseFromEnd)
      (:Update
        (Rendering|Material|SetScalarParameterValue _returnvalue "Opacity" _opacity_track :!class /Script/Engine.MaterialInstanceDynamic)))
    (else
      (Default|ToggleBlackScreen _asvrpawn)
      (Timeline|Opacity PlayFromStart))))

(event Custom|teleportPlayerToCage
  (bind _returnvalue (Game|Player|GetPlayerPawn 0))
  ;[0.1651 0.1651 0.1651] Helper Events
  (Utilities|Casting|CastToVRPawn _returnvalue)
  (CallFunction|AnimateBlackScreen)
  (Utilities|FlowControl|Delay 2.0)
  (Transformation|SetActorLocationAndRotation _returnvalue "1600.000000,3445.000000,-680.000000" "0.000000,-120.000000,0.000000" false true)
  (Utilities|FlowControl|Delay 2.0)
  (CallFunction|AnimateBlackScreen)
  (Input|EnableInput _returnvalue 0)
  (bind _asvrpawn (Utilities|Casting|CastToVRPawn _returnvalue))
  (Default|EnableWalkingSound _asvrpawn)
  (Utilities|FlowControl|Delay 12.0)
  (CallFunction|EndSequence))

(event Collision|EventActorBeginOverlap
  (params (OtherActor :type Actor%20Object%20Reference))
  ;[1 1 1] onTriggerOverlap
  (if (== OtherActor (Game|Player|GetPlayerPawn 0))
    (if (not (Variables|Default|GetisCageTriggered))
      (Utilities|FlowControl|Sequence
        (:then_0
          (CallFunction|PlayJumpScare)
          (Utilities|FlowControl|Delay 3.65)
          (CallFunction|TeleportPlayertoCage)
          (Utilities|UpdateHintText "Thanks for playing 
this demo!"))
        (:then_1
          (bind _cameranim (Timeline|Timeline PlayFromStart)
            (:Update
              (Transformation|SetActorRelativeRotation (Game|Player|GetPlayerPawn 0) (Math|Rotator|MakeRotator 0.0 0.0 (* (Variables|Default|GetrotationOfPlayerHead) _cameranim))))))))))

(fn ConstructionScript)