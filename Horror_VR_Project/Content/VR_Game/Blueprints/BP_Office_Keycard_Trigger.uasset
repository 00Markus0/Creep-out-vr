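; BP_Office_Keycard_Trigger is a trigger actor that handles the player picking up the office keycard in the VR game.
; On first successful player overlap, it validates its key, basement door and creep references, then passes the door and creep to the key and plays a piano sound.
; If the cage door is valid, it highlights that reader, sets the one-shot flag and updates the hint, whose callback moves the creep randomly.
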(event Collision|EventActorBeginOverlap
  (params (OtherActor :type Actor%20Object%20Reference))
  ;[1 1 1] Office Keycard picked up
  (if (== OtherActor (Game|Player|GetPlayerPawn 0))
    (if (not (Variables|Default|GetisStudyRoomKeycardPickedUp))
      (bind _officekeyreference (Variables|Default|GetofficeKeyReference)
        (:then
          (bind _basementdoorreference (Variables|Default|GetbasementDoorReference)
            (:then
              (bind _creeprefernce (Variables|Default|GetCreepRefernce)
                (:then
                  (Default|OfficeKeyPickedUp _officekeyreference _basementdoorreference _creeprefernce)
                  (Audio|PlaySoundatLocation "/Game/VR_Game/Sounds/S_Piano.S_Piano" "-450.000000,40.000000,0.000000" "0, 0, 0" 1.0 1.0 0.0 0 0 0 0)
                  (bind _cagedoorreference (Variables|Default|GetcageDoorReference)
                    (:then
                      (Default|HighlightReader _cagedoorreference)
                      (Variables|Default|SetisStudyRoomKeycardPickedUp true)
                      (Utilities|UpdateHintText "Don't get catched!"
                        (:updated
                          (Default|MovetoRandomLocation (Variables|Default|GetCreepRefernce)))))
                    (:else)))
                (:else)))
            (:else)))
        (:else)))))

(fn ConstructionScript)