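; B_LightSwitch is a one-time VR light switch that turns on the level lights and advances the objective to finding a keycard.
; An overlap on its trigger by any actor other than the player character toggles the target spot and point lights' visibility and plays a button sound.
; It then moves the highlight from the switch to the keycard and updates the hint text, with a boolean blocking repeat activation.
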(event OnComponentBeginOverlap(LightSwitchTrigger)
  (params (OverlappedComponent :type Primitive%20Component%20Object%20Reference) (OtherActor :type Actor%20Object%20Reference) (OtherComp :type Primitive%20Component%20Object%20Reference) (OtherBodyIndex :type Integer) (bFromSweep :type Boolean) (SweepResult :type Hit%20Result%20Structure%20%28by%20ref%29))
  ;[1 1 1] Enable Lights once
  (if (not (== OtherActor (Game|GetPlayerCharacter 0)))
    (if (not (Variables|Default|GetisLightSwitchOn))
      (CallFunction|UnHighlightLightSwitch)
      (Default|HighlightKeycard (Variables|Default|GetkeycardToHighlight))
      (Audio|PlaySound2D "/Game/HorrorEngine/Audio/_ReferenceCues/ButtonOn05_Ref.ButtonOn05_Ref" 1.0 1.0 0.0 0 0)
      (Rendering|ToggleVisibility (Variables|/Script/Engine.SpotLight|GetSpotLightComponent (Variables|Default|GetSpotLightTarget)) false)
      (for _array_element (Variables|Default|GetPointLightTarget)
        (Rendering|ToggleVisibility (Variables|/Script/Engine.PointLight|GetPointLightComponent _array_element) false))
      (Variables|Default|SetisLightSwitchOn true)
      (Utilities|UpdateHintText "Look out for 
a keycard!"))))

(event Custom|highlightLightSwitch
  ;[1 1 1] Highlight / Unhighlight LightSwitch
  (Rendering|SetVisibility (Variables|Default|GetHighlight) true false))

(event Custom|unHighlightLightSwitch
  ;[1 1 1] Highlight / Unhighlight LightSwitch
  (Rendering|SetVisibility (Variables|Default|GetHighlight) false false))

(event EventBeginPlay)

(event Collision|EventActorBeginOverlap
  (params (OtherActor :type Actor%20Object%20Reference)))

(event EventTick
  (params (DeltaSeconds :type Float%20%28single-precision%29)))

(fn ConstructionScript)