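; BP_Glass_Door is a lockable glass door that swings open on a timeline-driven yaw rotation.
; Overlapping LockBox with its assigned key unlocks it, cracks it ajar and adds an audio component.
; DoorOpenBox overlaps open it fully when CheckDoorOverlap passes.
; After a key unlock, a delayed player check can also open it, then highlight a linked light switch and update the hint text.
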(event OnComponentBeginOverlap(doorOpenBox)
  (params (OverlappedComponent :type Primitive%20Component%20Object%20Reference) (OtherActor :type Actor%20Object%20Reference) (OtherComp :type Primitive%20Component%20Object%20Reference) (OtherBodyIndex :type Integer) (bFromSweep :type Boolean) (SweepResult :type Hit%20Result%20Structure%20%28by%20ref%29))
  ;[1 1 1] Door Collision
  (Utilities|CheckDoorOverlap (Variables|Default|GetisDoorUnlocked) OtherActor (Variables|Default|GetcurrentRotation)
    (:Success
      (CallFunction|RotateDoor -9e+01))
    (:Failed
      (Development|PrintString "No overlap"))))

(event OnComponentBeginOverlap(lockBox)
  (params (OverlappedComponent :type Primitive%20Component%20Object%20Reference) (OtherActor :type Actor%20Object%20Reference) (OtherComp :type Primitive%20Component%20Object%20Reference) (OtherBodyIndex :type Integer) (bFromSweep :type Boolean) (SweepResult :type Hit%20Result%20Structure%20%28by%20ref%29))
  (bind _lightswitchtohighlight (Variables|Default|GetlightSwitchToHighlight))
  ;[1 1 1] unlock with key
  (Utilities|IsValid OtherActor
    (:Is%20Valid
      (if (== OtherActor (Variables|Default|GetkeyToUnlock))
        (if (not (Variables|Default|GetisDoorUnlocked))
          (CallFunction|UnlockDoor)
          (Utilities|FlowControl|Delay 0.65)
          (Utilities|CheckDoorOverlap true (Game|Player|GetPlayerPawn 0) (Variables|Default|GetcurrentRotation)
            (:Success
              (CallFunction|RotateDoor -9e+01)
              (Utilities|IsValid _lightswitchtohighlight
                (:Is%20Valid
                  (Default|HighlightLightSwitch _lightswitchtohighlight)
                  (Utilities|UpdateHintText "Explore"))))))))))

(event Custom|unlock%20Door
  ;[1 1 1] unlock Door
  (Variables|Default|SetisDoorUnlocked true)
  (CallFunction|RotateDoor -13.0)
  (AddComponent|AddAudioComponent false))

(event Custom|rotateDoor
  (params (rotation :type Float%20%28double-precision%29))
  ;[1 1 1] rotate Door
  (Variables|Default|SetcurrentRotation rotation)
  (bind _dooropenanim (Timeline|doorOpenAnim PlayFromStart)
    (:Update
      (Transformation|SetRelativeRotation (Variables|Default|GetSM_Door) (Math|Rotator|MakeRotator 0.0 0.0 (* _dooropenanim rotation)) false false))))

(event EventBeginPlay
  (bind _initalrotation (Variables|Default|GetinitalRotation))
  ;[1 1 1] Initialize door
  (if (Variables|Default|GetisDoorUnlocked)
    (CallFunction|RotateDoor _initalrotation)
    (Variables|Default|SetcurrentRotation _initalrotation)))

(fn ConstructionScript)