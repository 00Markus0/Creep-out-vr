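; B_Keycard is a keycard pickup for the VR game that toggles a Highlight component to draw attention to itself.
; On BeginPlay a flag decides whether the highlight starts visible.
; The office pickup event hides the highlight, rotates and unlocks the passed basement door, then teleports the wandering creep to a hardcoded position if both references are valid.
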(event Custom|officeKeyPickedUp
  (params (doorToBasement :type BP%20Door%20Object%20Reference%20%28by%20ref%29) (WanderingCreep :type BP%20Creep%20Chase%20Object%20Reference%20%28by%20ref%29))
  ;[1 1 1] Office
  (CallFunction|UnHighlightKeycard)
  (Utilities|IsValid doorToBasement
    (:Is%20Valid
      (Default|RotateDoor doorToBasement -22.0)
      (Variables|/Game/VR_Game/Blueprints/BP_Door.BP_Door_C|SetisDoorUnlocked doorToBasement true)
      (Utilities|IsValid WanderingCreep
        (:Is%20Valid
          (Transformation|SetActorLocationAndRotation WanderingCreep "55.000000,800.000000,96.000000" "0.000000,180.000000,0.000000" false true))))))

(event Custom|highlightKeycard
  ;[1 1 1] Highlight / Unhighlight Key
  (Rendering|SetVisibility (Variables|Default|GetHighlight) true false))

(event Custom|unHighlightKeycard
  ;[1 1 1] Highlight / Unhighlight Key
  (Rendering|SetVisibility (Variables|Default|GetHighlight) false false))

(event EventBeginPlay
  (if (Variables|Default|GetisHighlitedAtStart)
    (CallFunction|HighlightKeycard)
    (else
      (CallFunction|UnHighlightKeycard))))

(fn ConstructionScript)